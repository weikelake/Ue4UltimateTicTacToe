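; BP_bigGrid is the board manager for what appears to be nested tic-tac-toe, built from nine small BP_grid boards.
; On BeginPlay it spawns them in a 3x3 layout and fills the GameInstance's BigCellsXO with -1 (open).
; ClearTB records the previous grid, disables all boards, then enables the CurrentGrid board, or every open board if that one is closed.
; Chrome material marks playable boards, pine wood the rest.
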(event Custom|ClearTB
  (params (grid :type BP%20Grid%20Object%20Reference))
  (bind _as_gi (Variables|Default|GetAs%20GI))
  (bind _arraygrids (Variables|Default|GetarrayGrids))
  (bind _as_gi_2 (Variables|Default|GetAs%20GI))
  (bind _currentgrid (Variables|/Game/core/GI.GI_C|GetcurrentGrid _as_gi_2))
  (bind _output (Utilities|Array|Get(acopy) _arraygrids _currentgrid))
  (for (_array_element _array_index) (Variables|Default|GetarrayGrids)
    (if (== grid _array_element)
      (Variables|Default|SetprevGrid _array_index)))
  (for _array_element_2 (Variables|Default|GetarrayGrids)
    (Default|SetBindEventforAllCells _array_element_2 false)
    (for _index (range 0 7)
      (Rendering|Material|SetMaterial (Variables|/Game/BPs/BP_grid.BP_grid_C|GetSM_grid _array_element_2) _index "/Game/texturesAndMaterials/T_Wood_Pine_Mat.T_Wood_Pine_Mat")))
  (if (!= (Utilities|Array|Get(acopy) (Variables|/Game/core/GI.GI_C|GetbigCellsXO _as_gi) (Variables|/Game/core/GI.GI_C|GetcurrentGrid _as_gi)) -1)
    (for (_array_element_3 _array_index_2) (Variables|Default|GetarrayGrids)
      (if (not (!= (Utilities|Array|Get(acopy) (Variables|/Game/core/GI.GI_C|GetbigCellsXO (Variables|Default|GetAs%20GI)) _array_index_2) -1))
        (Default|SetBindEventforAllCells _array_element_3 true)
        (for _index_2 (range 0 7)
          (Rendering|Material|SetMaterial (Variables|/Game/BPs/BP_grid.BP_grid_C|GetSM_grid _array_element_3) _index_2 "/Game/texturesAndMaterials/M_Metal_Chrome.M_Metal_Chrome"))))
    (else
      (Default|SetBindEventforAllCells _output true)
      (for _index_3 (range 0 7)
        (Rendering|Material|SetMaterial (Variables|/Game/BPs/BP_grid.BP_grid_C|GetSM_grid _output) _index_3 "/Game/texturesAndMaterials/M_Metal_Chrome.M_Metal_Chrome")))))

(event EventBeginPlay
  (Utilities|SpawnGrids
    (:Out
      (bind _asgi (Utilities|Casting|CastToGI (Game|GetGameInstance)))
      (Variables|Default|SetAs%20GI _asgi)
      (for _index (range 0 8)
        (Utilities|Array|Insert (Variables|/Game/core/GI.GI_C|GetbigCellsXO (Variables|Default|GetAs%20GI)) -1 _index)))))

(fn ConstructionScript)